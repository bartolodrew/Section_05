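; AI controller for guard NPCs that runs the GuardBehaviour behavior tree on the PatrolData blackboard from BeginPlay.
; AI Perception updates write any sensed actor without the "Enemy" tag to the EnemyKey blackboard entry.
; When such an actor stops being sensed, the key is cleared; actors tagged "Enemy" are ignored.
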(event `self.ReceiveBeginPlay`
  (bind _blackboardcomponent (`self.UseBlackboard` "/Game/Static/NPC/AI/PatrolData.PatrolData"))
  (`self.RunBehaviorTree` "/Game/Static/NPC/AI/GuardBehaviour.GuardBehaviour")
  (set `self.BlackboardComp` _blackboardcomponent))

(event `self.AIPerception.OnTargetPerceptionUpdated`
  (params (Actor :type "Actor Object Reference") (Stimulus :type "AIStimulus Structure"))
  (bind _blackboardcomp (`self.BlackboardComp`))
  (if (`self.ActorHasTag` Actor "Enemy")
    _
    (elif (`.bSuccessfullySensed` (break `AIStimulus` Stimulus))
      (`BlackboardComponent.SetValueAsObject` _blackboardcomp (`self.EnemyKey`) Actor)
      (else
        (`BlackboardComponent.ClearValue` _blackboardcomp (`self.EnemyKey`))))))

(fn `UserConstructionScript`)
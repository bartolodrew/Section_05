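; NPC AI controller that runs the Patrol behavior tree on the PatrolData blackboard.
; Every tick it writes player pawn 0 into the blackboard's enemy key, regardless of what is perceived.
; AI Perception updates only print the controlled pawn, the sense class and the perceived actor, without feeding the blackboard.
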(event `self.ReceiveBeginPlay`
  (bind _blackboardcomponent (`self.UseBlackboard` "/Game/NPC/AI/PatrolData.PatrolData"))
  (`self.RunBehaviorTree` "/Game/NPC/AI/Patrol.Patrol")
  (set `self.BlackboardComp` _blackboardcomponent))

(event `self.ReceiveTick`
  (params (DeltaSeconds :type "Float (single-precision)"))
  (`BlackboardComponent.SetValueAsObject` (`self.BlackboardComp`) (`self.EnemyKey`) (`GameplayStatics.GetPlayerPawn` 0)))

(event `self.AIPerception.OnTargetPerceptionUpdated`
  (params (Actor :type "Actor Object Reference") (Stimulus :type "AIStimulus Structure"))
  (bind _returnvalue (`AIPerceptionSystem.GetSenseClassForStimulus` Stimulus))
  (`KismetSystemLibrary.PrintString` (`KismetStringLibrary.Concat_StrStr` (`KismetSystemLibrary.GetObjectName` (`self.K2_GetPawn`)) " " (`KismetSystemLibrary.GetClassDisplayName` _returnvalue) " " (`KismetSystemLibrary.GetObjectName` Actor))))

(fn `UserConstructionScript`)